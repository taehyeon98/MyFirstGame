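; BP_SingleCannon is a child cannon Blueprint with a limited ammo count, fired through the CannonFire event.
; ShootCannon calls the parent shot while Count remains, decrements it and pushes it to a CountWidget, otherwise printing a red out-of-ammo message in Korean.
; Each Tick, UpdateLookCamera turns the widget component toward the player camera using only X and Y, so it rotates in yaw without tilting.
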(event EventCannonFire
  (CallFunction|ShootCannon))

(event EventTick
  (params (DeltaSeconds :type Float%20%28single-precision%29))
  (CallFunction|UpdateLookCamera))

(fn ConstructionScript
  (|CallParentFunction))

(fn ShootCannon
  (if (> (Variables|Default|GetCount) 0)
    (|CallParentFunction)
    (Variables|Default|SetCount (- (Variables|Default|GetCount) 1))
    (bind _ascount_widget (Utilities|Casting|CastToCountWidget (UserInterface|GetUserWidgetObject (Variables|Default|GetWidget))))
    (Default|SetCount _ascount_widget (Variables|Default|GetCount))
    (else
      (Development|PrintString "대포알이 없습니다." true true "(R=1.000000,G=0.000000,B=0.065514,A=1.000000)"))))

(fn UpdateLookCamera
  (bind _returnvalue (Game|GetPlayerCameraManager 0))
  (bind _widget (Variables|Default|GetWidget))
  (bind _returnvalue_2 (Transformation|GetWorldLocation _widget))
  (bind _returnvalue_3 (Transformation|GetActorLocation _returnvalue))
  (Transformation|SetWorldRotation (Variables|Default|GetWidget) (Math|Rotator|FindLookatRotation (Math|Vector|MakeVector (.x _returnvalue_2) (.y _returnvalue_2) 0.0) (Math|Vector|MakeVector (.x _returnvalue_3) (.y _returnvalue_3) 0.0)) false false))